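; BP_SizeChanger is a painter interactable that changes a controller's size when interacted with.
; BeginInteraction multiplies the controller's CurrentSize by SizeMultiplier and applies it through SetSize.
; It also carries tool functions that name it "Block" and spawn a BP_Brush_Block initialized with the controller, separate from the resize logic.
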(event EventBeginInteraction
  (params (ControllerActor :type Painter%20Controller%20Object%20Reference))
  (Default|SetSize ControllerActor (* (Variables|/Game/PawnAndController/PainterController.PainterController_C|GetCurrentSize ControllerActor) (Variables|Default|GetSizeMultiplier))))

(fn ConstructionScript)

(fn CreateBrushfromTool
  (params (Controller :type Painter%20Controller%20Object%20Reference))
  (bind _returnvalue (Game|SpawnActorfromClass "/Game/Painter/BP_Brush_Block.BP_Brush_Block_C" (Math|Transform|MakeTransform "0, 0, 0") "AlwaysSpawn" 0 0))
  (Default|InitBrush _returnvalue Controller)
  (return _returnvalue))

(fn GetToolName
  (return "Block"))