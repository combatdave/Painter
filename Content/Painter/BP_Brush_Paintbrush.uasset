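; Paintbrush for a painting tool that draws a tube-shaped stroke along the controller cursor's path, using the controller's color, material and size captured at init.
; Each tick it records a new point once the cursor moves past a distance threshold.
; Each point triggers a full procedural mesh rebuild: vertex rings oriented toward the next point are stitched into triangles, then given a dynamic material instance tinted with the color.
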(event EventTickBrush
  (params (Controller :type Painter%20Controller%20Object%20Reference))
  (bind _cursor (Variables|/Game/PawnAndController/PainterController.PainterController_C|GetCursor Controller))
  (bind _returnvalue (Transformation|GetWorldLocation _cursor))
  (if (|ShouldCreatePoint _returnvalue)
    (CallFunction|CreateNewPoint _returnvalue)))

(event EventInitBrush
  (params (Controller :type Painter%20Controller%20Object%20Reference))
  (Variables|Default|SetColor (Variables|/Game/PawnAndController/PainterController.PainterController_C|GetCurrentColor Controller))
  (Variables|Default|SetMaterial (Variables|/Game/PawnAndController/PainterController.PainterController_C|GetCurrentMaterial Controller))
  (Variables|Default|SetRadius (Variables|/Game/PawnAndController/PainterController.PainterController_C|GetCurrentSize Controller)))

(fn ConstructionScript)

(fn CreateNewPoint
  (params (Location :type Vector))
  (Utilities|Array|Add (Variables|Default|GetLocations) Location)
  (CallFunction|GenerateVertices)
  (CallFunction|UpdateMeshwithVertices))

(fn GenerateVertices
  (Utilities|Array|Clear (Variables|Default|GetVertices))
  (Utilities|Array|Clear (Variables|Default|GetNormals))
  (for (_array_element _array_index) (Variables|Default|GetLocations)
    (if (|HasNextPoint _array_index)
      (for _index (range 0 (- (Variables|Default|GetNumVertsPerLoop) 1))
        (Utilities|Array|Add (Variables|Default|GetVertices) (.Vertex (|GetVertexForIndex _index (Math|Transform|MakeTransform "0, 0, 0" (Math|Rotator|MakeRotfromXZ (|GetDirectionToNextLocation _array_index _array_element) (Math|Vector|MakeVector 0.0 0.0 1.0))) _array_element)))
        (Utilities|Array|Add (Variables|Default|GetNormals) (.Normal (|GetVertexForIndex _index (Math|Transform|MakeTransform "0, 0, 0" (Math|Rotator|MakeRotfromXZ (|GetDirectionToNextLocation _array_index _array_element) (Math|Vector|MakeVector 0.0 0.0 1.0))) _array_element)))))))

(fn UpdateMeshwithVertices
  (bind _proceduralmesh (Variables|Default|GetProceduralMesh))
  (Class|ProceduralMeshComponent|ClearMeshSection (Variables|Default|GetProceduralMesh))
  (CallFunction|GenerateTriangles)
  (Class|ProceduralMeshComponent|CreateMeshSection (Variables|Default|GetProceduralMesh) 0 (Variables|Default|GetVertices) (Variables|Default|GetTriangles) (Variables|Default|GetNormals) 0 0 0 false)
  (bind _returnvalue (Rendering|Material|CreateDynamicMaterialInstance _proceduralmesh 0 (Variables|Default|GetMaterial) :!class /Script/Engine.PrimitiveComponent))
  (Rendering|Material|SetVectorParameterValue _returnvalue "Color" (Variables|Default|GetColor) :!class /Script/Engine.MaterialInstanceDynamic)
  (Rendering|Material|SetMaterial _proceduralmesh 0 _returnvalue))

(fn GenerateTriangles
  (bind _triangles (Variables|Default|GetTriangles))
  (bind _numvertsperloop (Variables|Default|GetNumVertsPerLoop))
  (bind _triangles_2 (Variables|Default|GetTriangles))
  (Utilities|Array|Clear (Variables|Default|GetTriangles))
  (for _index (range 0 (- (/ (Utilities|Array|Length (Variables|Default|GetVertices)) (Variables|Default|GetNumVertsPerLoop)) 1))
    (for _index_2 (range 0 (- (Variables|Default|GetNumVertsPerLoop) 1))
      (Utilities|FlowControl|Sequence
        (:then_0
          (Utilities|FlowControl|Sequence
            (:then_0
              (Utilities|Array|Add _triangles (+ _index_2 (* _index (Variables|Default|GetNumVertsPerLoop)))))
            (:then_1
              (Utilities|Array|Add _triangles (+ (+ _index_2 (* _index (Variables|Default|GetNumVertsPerLoop))) (Variables|Default|GetNumVertsPerLoop))))
            (:then_2
              (Utilities|Array|Add _triangles (+ (+ _index_2 (* _index (Variables|Default|GetNumVertsPerLoop))) 1)))))
        (:then_1
          (Utilities|FlowControl|Sequence
            (:then_0
              (Utilities|Array|Add _triangles_2 (+ (+ _index_2 (* _index (Variables|Default|GetNumVertsPerLoop))) _numvertsperloop)))
            (:then_1
              (Utilities|Array|Add _triangles_2 (+ (+ _index_2 (* _index (Variables|Default|GetNumVertsPerLoop))) (+ _numvertsperloop 1))))
            (:then_2
              (Utilities|Array|Add _triangles_2 (+ (+ _index_2 (* _index (Variables|Default|GetNumVertsPerLoop))) 1)))))))))