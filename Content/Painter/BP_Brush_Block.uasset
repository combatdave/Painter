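; BP_Brush_Block is a painter brush that lays down cube blocks at the controller's cursor.
; InitBrush scales the actor by the current size, applies a dynamic instance of the current material with a randomly varied current color, and moves it to the cursor.
; TickBrush spawns and initializes further copies of its own class at a timed interval, so one brush actor emits a trail of blocks.
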(event EventInitBrush
  (params (Controller :type Painter%20Controller%20Object%20Reference))
  (bind _currentsize (Variables|/Game/PawnAndController/PainterController.PainterController_C|GetCurrentSize Controller))
  (Transformation|SetActorScale3D (Math|Vector|MakeVector _currentsize _currentsize _currentsize))
  (bind _returnvalue (Rendering|Material|CreateDynamicMaterialInstance (Variables|Default|GetCube) 0 (Variables|/Game/PawnAndController/PainterController.PainterController_C|GetCurrentMaterial Controller) :!class /Script/Engine.PrimitiveComponent))
  (Rendering|Material|SetVectorParameterValue _returnvalue "Color" (* (Variables|/Game/PawnAndController/PainterController.PainterController_C|GetCurrentColor Controller) (Math|Random|RandomFloatinRange 0.8 1.2)) :!class /Script/Engine.MaterialInstanceDynamic)
  (Transformation|SetActorLocation (Transformation|GetWorldLocation (Variables|/Game/PawnAndController/PainterController.PainterController_C|GetCursor Controller)) false false)
  (Variables|Default|SetNextSpawnTime (+ (Utilities|Time|GetGameTimeinSeconds) (Variables|Default|GetTimeBetweenBlocks))))

(event EventTickBrush
  (params (Controller :type Painter%20Controller%20Object%20Reference))
  (if (> (Utilities|Time|GetGameTimeinSeconds) (Variables|Default|GetNextSpawnTime))
    (bind _returnvalue (Game|SpawnActorfromClass "BP_Brush_Block_C" (Math|Transform|MakeTransform "0, 0, 0") "Undefined" 0 0))
    (CallFunction|InitBrush _returnvalue Controller)
    (Variables|Default|SetNextSpawnTime (+ (Utilities|Time|GetGameTimeinSeconds) (Variables|Default|GetTimeBetweenBlocks)))))

(fn ConstructionScript)